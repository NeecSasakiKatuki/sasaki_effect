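; BP_woodtran is a moving floor actor in the tutorial folder that shuttles back and forth along the world Y axis.
; BeginPlay records the start location, and Tick offsets the actor by Speed without sweep, flipping Speed's direction when it passes the start or a fixed distance beyond it.
; Movement is a fixed step per frame, not scaled by delta time, so its speed follows frame rate.
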(event EventBeginPlay
  (Variables|Default|Setstart%20location (Transformation|GetActorLocation)))

(event Collision|EventActorBeginOverlap
  (params (OtherActor :type Actor%20Object%20Reference)))

(event EventTick
  (params (DeltaSeconds :type Float%20%28single-precision%29))
  ;[1 1 1] 床移動
  (Transformation|AddActorWorldOffset (Variables|Default|Getspeed))
  (if (> (.y (Transformation|GetActorLocation)) (+ (.y (Variables|Default|Getstart%20location)) 1.7e+03))
    (Variables|Default|Setspeed "0,-10.000000, 0")
    (elif (< (.y (Transformation|GetActorLocation)) (.y (Variables|Default|Getstart%20location)))
      (Variables|Default|Setspeed "0,10.000000, 0"))))

(fn ConstructionScript)